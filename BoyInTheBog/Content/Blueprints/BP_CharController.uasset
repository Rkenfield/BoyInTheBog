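; BP_CharController is a player controller that toggles a pause menu widget from the Pause input action.
; Opening creates the widget, adds it to the viewport and switches to Game and UI input; closing removes it, and only the Paused flag tracks state.
; ResumeGame removes the widget through the PauseMenu variable, which opening sets to None.
; Game time is never paused, and input mode is never restored.
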(event `InputAction|Pause`
  (params (Key :type "Key Structure"))
  (:`Pressed`
    (if (`self.Paused`)
      (`Widget.RemoveFromParent` (stale _returnvalue))
      (set `self.Paused` false)
      (else
        (bind _returnvalue (`|CreateWidget` "/Game/Blueprints/Widgets/PauseMenu.PauseMenu_C"))
        (set `self.PauseMenu` null)
        (`UserWidget.AddToViewport` _returnvalue 0)
        (set `self.Paused` true)
        (`WidgetBlueprintLibrary.SetInputMode_GameAndUIEx` self _returnvalue)))))

(fn `Resume Game`
  (`Widget.RemoveFromParent` (`self.PauseMenu`))
  (set `self.Paused` false))

(fn `UserConstructionScript`)
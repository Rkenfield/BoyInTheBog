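; Drivable raft pawn that the player's BP_Boy can board through the ControlBoatBox trigger, which toggles CanBoat.
; While possessed, Tick pins the hidden Boy above the box, eases the raft's yaw toward camera-relative input and moves it forward by BoatSpeed per frame, unscaled by delta time.
; Interact calls PossesBoy to hide the stand-in player, restore Boy's visibility and collision, and return possession to him.
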(event `self.ReceiveBeginPlay`
  (bind _returnvalue (`GameplayStatics.GetActorOfClass` "/Game/Blueprints/BP_Boy.BP_Boy_C"))
  (set `self.Boy` _returnvalue))

(event `self.ReceiveTick`
  (params (DeltaSeconds :type "Float (single-precision)"))
  (bind _raft (`self.Raft`))
  (bind (_returnvalue_x _returnvalue_y _returnvalue_z) (`KismetMathLibrary.BreakVector` (`SceneComponent.K2_GetComponentLocation` (`self.ControlBoatBox`))))
  (bind (_returnvalue_roll _returnvalue_pitch _returnvalue_yaw) (`KismetMathLibrary.BreakRotator` (`SceneComponent.K2_GetComponentRotation` _raft)))
  (bind (_returnvalue_roll_2 _returnvalue_pitch_2 _returnvalue_yaw_2) (`KismetMathLibrary.BreakRotator` (`KismetMathLibrary.RInterpTo` (`KismetMathLibrary.MakeRotator` _returnvalue_roll _returnvalue_pitch _returnvalue_yaw) (`KismetMathLibrary.MakeRotFromX` (`self.MoveDirection`)) DeltaSeconds 1.0)))
  (if (`self.isPosessed`)
    (`self.K2_SetActorLocation` (`self.Boy`) (`KismetMathLibrary.MakeVector` _returnvalue_x _returnvalue_y (+ _returnvalue_z 100.0)) false true)
    (if (or (!= (`self.GetInputAxisValue`) 0.0) (!= (`self.GetInputAxisValue`) 0.0))
      (set `self.MoveDirection` (`KismetMathLibrary.Normal` (+ (`self.ForwardInput`) (`self.RightInput`))))
      (`SceneComponent.K2_SetRelativeRotation` _raft (`KismetMathLibrary.MakeRotator` _returnvalue_roll _returnvalue_pitch _returnvalue_yaw_2) false false)
      (`self.K2_SetActorLocation` (+ (* (`SceneComponent.GetForwardVector` (`self.Raft`)) (`self.BoatSpeed`)) (`self.K2_GetActorLocation`)))
      (else
        (set `self.MoveDirection` (0.0 0.0 0.0))))))

(event `InputAxis|Forward/Backward`
  (params (AxisValue :type "Float (single-precision)"))
  (bind (_returnvalue_x _returnvalue_y) (`KismetMathLibrary.BreakVector` (`SceneComponent.GetForwardVector` (`self.SpringArm`))))
  (set `self.ForwardInput` (* (`KismetMathLibrary.MakeVector` _returnvalue_x _returnvalue_y) AxisValue)))

(event `InputAxis|Left/Right`
  (params (AxisValue :type "Float (single-precision)"))
  (bind (_returnvalue_x _returnvalue_y) (`KismetMathLibrary.BreakVector` (`SceneComponent.GetRightVector` (`self.SpringArm`))))
  (set `self.RightInput` (* (`KismetMathLibrary.MakeVector` _returnvalue_x _returnvalue_y) AxisValue)))

(event `self.ControlBoatBox.OnComponentBeginOverlap`
  (params (OverlappedComponent :type "PrimitiveComponent Object Reference") (OtherActor :type "Actor Object Reference") (OtherComp :type "PrimitiveComponent Object Reference") (OtherBodyIndex :type Integer) (bFromSweep :type Boolean) (SweepResult :type "HitResult Structure (by ref)"))
  (bind _asbp_boy (cast `/Game/Blueprints/BP_Boy` OtherActor))
  (set `/Game/Blueprints/BP_Boy.CanBoat` true _asbp_boy))

(event `self.ControlBoatBox.OnComponentEndOverlap`
  (params (OverlappedComponent :type "PrimitiveComponent Object Reference") (OtherActor :type "Actor Object Reference") (OtherComp :type "PrimitiveComponent Object Reference") (OtherBodyIndex :type Integer))
  (bind _asbp_boy (cast `/Game/Blueprints/BP_Boy` OtherActor))
  (set `/Game/Blueprints/BP_Boy.CanBoat` false _asbp_boy))

(event `self.ReceivePossessed`
  (params (NewController :type "Controller Object Reference")))

(event `InputAction|Interact`
  (params (Key :type "Key Structure"))
  (:`Pressed`
    (set `/Game/Blueprints/BP_Boy.CanBoat` false (`self.Boy`))
    (`self.PossesBoy`)
    (set `self.isPosessed` false)))

(fn `PossesBoy`
  (bind _boy (`self.Boy`))
  (`|ExecutionSequence`
    (:`then_0`
      (`PrimitiveComponent.SetCollisionEnabled` (`self.ControlBoatBox`) "QueryOnly"))
    (:`then_1`
      (`PrimitiveComponent.SetCollisionEnabled` (`Character.CapsuleComponent` (`self.Boy`)) "QueryAndPhysics"))
    (:`then_2`
      (`SceneComponent.SetVisibility` (`self.TempFakePlayer`) false true)
      (`SceneComponent.SetVisibility` (`Actor.RootComponent` _boy) true true)
      (set `/Game/Blueprints/BP_Boy.inBoat` false _boy))
    (:`then_3`
      (`Controller.Possess` (`GameplayStatics.GetPlayerController` 0) (`self.Boy`))
      (set `self.isPosessed` false))))

(fn `UserConstructionScript`
  (`SceneComponent.SetAbsolute` (`self.SpringArm`) false true false))
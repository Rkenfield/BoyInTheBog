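; BobberTransfer is a fishing bobber actor that decides whether a cast has landed in water.
; When its Box overlaps a WaterPlane, it sets the boy to fishing, spawns a BobberEnd at its Cube's location, cross-links that with the boy and destroys itself.
; Overlapping anything else except itself or the boy, before a success, clears fishing, restores the boy's movement and destroys the bobber.
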(event `self.ReceiveTick`
  (params (DeltaSeconds :type "Float (single-precision)")))

(event `self.Box.OnComponentBeginOverlap`
  (params (OverlappedComponent :type "PrimitiveComponent Object Reference") (OtherActor :type "Actor Object Reference") (OtherComp :type "PrimitiveComponent Object Reference") (OtherBodyIndex :type Integer) (bFromSweep :type Boolean) (SweepResult :type "HitResult Structure (by ref)"))
  (bind _boyref (`self.BoyRef`))
  (bind _success (`self.success`))
  (cast `/Game/Blueprints/WaterPlane` OtherActor
    (:`then`
      (set `/Game/Blueprints/BP_Boy.IsFishing` true _boyref)
      (set `self.success` true)
      (bind _returnvalue (`|SpawnActorFromClass` "/Game/Blueprints/BobberEnd.BobberEnd_C" (`KismetMathLibrary.MakeTransform` (`SceneComponent.K2_GetComponentLocation` (`self.Cube`))) "Undefined" "OverrideRootScale" null null))
      (bind _output_get (set `/Game/Blueprints/BobberEnd.BoyRef` (`self.BoyRef`) _returnvalue))
      (set `/Game/Blueprints/BP_Boy.BobberRef` _returnvalue _output_get)
      (`self.K2_DestroyActor`))
    (:`CastFailed`
      (if (and (!= OtherActor self) (!= OtherActor (`self.BoyRef`)) (not _success))
        (set `/Game/Blueprints/BP_Boy.IsFishing` false _boyref)
        (set `/Game/Blueprints/BP_Boy.CanMove` true _boyref)
        (`KismetSystemLibrary.PrintString` (`KismetStringLibrary.Conv_BoolToString` _success))
        (`self.K2_DestroyActor`)))))

(fn `UserConstructionScript`)
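; Player pawn for the fishing boy, handling camera-relative movement, aiming, casting, reeling and switching possession to the boat.
; Holding Cast charges a throw; releasing launches a BobberTransfer, and later presses reel the bobber in on a looping timer.
; StartHooked swaps to a fight loop where reel-axis input opposing the fish pulls it in, scaled by pole pull minus fish speed.
; Close fish join CaughtInventory; distant ones escape.
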(event `self.ReceiveBeginPlay`
  (bind _returnvalue (`GameplayStatics.GetActorOfClass` "/Game/Blueprints/BP_Boat.BP_Boat_C"))
  (set `self.Boat` _returnvalue)
  (bind _returnvalue_2 (`|GenericCreateObject` "/Game/Blueprints/FishingPoles/StarterPole.StarterPole_C" self))
  (set `self.CurrentPole` _returnvalue_2))

(event `self.ReceiveTick`
  (params (DeltaSeconds :type "Float (single-precision)"))
  (bind _returnvalue (`KismetMathLibrary.Normal` (+ (`self.ForwardInput`) (`self.RightInput`))))
  (if (`self.inBoat`)
    _
    (elif (and (or (!= (`self.GetInputAxisValue`) 0.0) (!= (`self.GetInputAxisValue`) 0.0)) (`self.CanMove`))
      (set `self.MoveDirection` _returnvalue)
      (if (`self.Aiming`)
        (`SceneComponent.K2_SetRelativeRotation` (`self.Cube`) (`KismetMathLibrary.MakeRotFromX` (`self.MoveDirection`)) false false)
        (else
          (`SceneComponent.K2_SetRelativeRotation` (`self.Cube`) (`KismetMathLibrary.MakeRotFromX` (`self.MoveDirection`)) false false)
          (`self.K2_SetActorLocation` (+ (* _returnvalue (`self.Speed`)) (`self.K2_GetActorLocation`)) true))))))

(event `InputAxis|Forward/Backward`
  (params (AxisValue :type "Float (single-precision)"))
  (bind (_returnvalue_x _returnvalue_y) (`KismetMathLibrary.BreakVector` (`SceneComponent.GetForwardVector` (`self.SpringArm`))))
  (set `self.ForwardInput` (* (`KismetMathLibrary.MakeVector` _returnvalue_x _returnvalue_y) AxisValue)))

(event `InputAxis|Left/Right`
  (params (AxisValue :type "Float (single-precision)"))
  (bind (_returnvalue_x _returnvalue_y) (`KismetMathLibrary.BreakVector` (`SceneComponent.GetRightVector` (`self.SpringArm`))))
  (set `self.RightInput` (* (`KismetMathLibrary.MakeVector` _returnvalue_x _returnvalue_y) AxisValue)))

(event `InputAction|Cast`
  (params (Key :type "Key Structure"))
  (:`Pressed`
    (if (`self.IsFishing`)
      (if (`KismetSystemLibrary.IsValid` (`self.BobberRef`))
        (if (not (`self.Hooked`))
          (bind _returnvalue (`KismetSystemLibrary.K2_SetTimer` null "Reel" 0.001 true))
          (set `self.ReelHandle` _returnvalue)))
      (else
        (set `self.CanMove` false)
        (bind _returnvalue_2 (`KismetSystemLibrary.K2_SetTimer` null "CastChargeUp" 0.1 true))
        (set `self.CastHandle` _returnvalue_2))))
  (:`Released`
    (if (`self.IsFishing`)
      (`KismetSystemLibrary.K2_ClearAndInvalidateTimerHandle` (`self.ReelHandle`))
      (elif (not (`self.CanMove`))
        (`KismetSystemLibrary.K2_ClearAndInvalidateTimerHandle` (`self.CastHandle`))
        (bind _returnvalue_3 (`|SpawnActorFromClass` "/Game/Blueprints/BobberTransfer.BobberTransfer_C" (`KismetMathLibrary.MakeTransform` (+ (0.0 0.0 100.0) (`self.K2_GetActorLocation`))) "Undefined" "OverrideRootScale" null null))
        (set `/Game/Blueprints/BobberTransfer.BoyRef` self _returnvalue_3)
        (`PrimitiveComponent.AddImpulse` (`/Game/Blueprints/BobberTransfer.Cube` _returnvalue_3) (* (`SceneComponent.GetForwardVector` (`self.Cube`)) (* (`self.CastCharge`) 1000.0)) "None" false)
        (set `self.CastCharge` 1.0)
        (set `self.IsFishing` true)))))

(event `InputAction|Aim`
  (params (Key :type "Key Structure"))
  (:`Pressed`
    (set `self.Aiming` true))
  (:`Released`
    (set `self.Aiming` false)))

(event `InputAction|Interact`
  (params (Key :type "Key Structure"))
  (:`Pressed`
    (if (`self.CanBoat`)
      (`self.PosessBoat`))))

(event `self.ReceivePossessed`
  (params (NewController :type "Controller Object Reference"))
  (bind (_returnvalue_x _returnvalue_y _returnvalue_z) (`KismetMathLibrary.BreakVector` (`SceneComponent.K2_GetComponentLocation` (`/Game/Blueprints/BP_Boat.ControlBoatBox` (`self.Boat`)))))
  (if (`KismetSystemLibrary.IsValid` (`self.Boat`))
    (`KismetSystemLibrary.Delay` 0.001)
    (`self.K2_SetActorLocation` (`KismetMathLibrary.MakeVector` _returnvalue_x _returnvalue_y (+ _returnvalue_z 100.0)) false true)))

(event `InputAxis|ReelBackward/Forward`
  (params (AxisValue :type "Float (single-precision)"))
  (bind (_returnvalue_x _returnvalue_y) (`KismetMathLibrary.BreakVector` (`SceneComponent.GetForwardVector` (`self.SpringArm`))))
  (set `self.ReelForward` (* (`KismetMathLibrary.MakeVector` _returnvalue_x _returnvalue_y) (* AxisValue -1.0))))

(event `InputAxis|ReelLeft/Right`
  (params (AxisValue :type "Float (single-precision)"))
  (bind (_returnvalue_x _returnvalue_y) (`KismetMathLibrary.BreakVector` (`SceneComponent.GetRightVector` (`self.SpringArm`))))
  (set `self.ReelRight` (* (`KismetMathLibrary.MakeVector` _returnvalue_x _returnvalue_y) AxisValue)))

(fn `CastChargeUp`
  (locals (ChargeUpAmount :type "Float (double-precision)") (ChargeCount :type "Float (double-precision)"))
  (if (< (`self.CastCharge`) 100.0)
    (set `self.CastCharge` (+ (`self.CastCharge`) 1.0))))

(fn `PosessBoat`
  (bind _boat (`self.Boat`))
  (`|ExecutionSequence`
    (:`then_0`
      (`SceneComponent.SetVisibility` (`self.CapsuleComponent`) false true))
    (:`then_1`
      (`SceneComponent.SetVisibility` (`/Game/Blueprints/BP_Boat.TempFakePlayer` (`self.Boat`)) true true))
    (:`then_2`
      (`PrimitiveComponent.SetCollisionEnabled` (`/Game/Blueprints/BP_Boat.ControlBoatBox` _boat) "NoCollision"))
    (:`then_3`
      (`Controller.Possess` (`GameplayStatics.GetPlayerController` 0) _boat)
      (set `/Game/Blueprints/BP_Boat.BoyRotation` (`self.MoveDirection`) _boat)
      (set `SceneComponent.bAbsoluteRotation` true (`self.Cube`))
      (set `/Game/Blueprints/BP_Boat.isPosessed` true _boat)
      (set `self.inBoat` true))))

(fn `Reel`
  (locals (ReelSpeedTemp :type "Float (double-precision)" :default 10.0))
  (bind _bobberref (`self.BobberRef`))
  (bind _returnvalue (`KismetMathLibrary.Vector_Distance` (`self.K2_GetActorLocation` (`self.BobberRef`)) (`self.K2_GetActorLocation`)))
  (bind (_returnvalue_x _returnvalue_y) (`KismetMathLibrary.BreakVector` (`KismetMathLibrary.Normal` (- (`self.K2_GetActorLocation`) (`self.K2_GetActorLocation` (`self.BobberRef`))))))
  (if (< _returnvalue 250.0)
    (set `self.ReelDirection` (`KismetMathLibrary.MakeVector` _returnvalue_x _returnvalue_y))
    (else
      (set `self.ReelDirection` (`KismetMathLibrary.Normal` (- (`self.K2_GetActorLocation`) (`self.K2_GetActorLocation` (`self.BobberRef`)))))))
  (if (<= _returnvalue 100.0)
    (`KismetSystemLibrary.K2_ClearAndInvalidateTimerHandle` (`self.ReelHandle`))
    (`self.K2_DestroyActor` (`self.BobberRef`))
    (set `self.IsFishing` false)
    (set `self.CanMove` true)
    (else
      (`self.K2_SetActorLocation` _bobberref (+ (`self.K2_GetActorLocation` _bobberref) (* (`self.ReelDirection`) (`/Game/Blueprints/FishingPoles/FishingPole.Pullspeed` (`self.CurrentPole`)))) false false))))

(fn `Reel Hooked`
  (locals (ReelDir :type "Vector Structure"))
  (bind (_returnvalue_x _returnvalue_y) (`KismetMathLibrary.BreakVector` (`self.K2_GetActorLocation`)))
  (bind _caughtinventory (`self.CaughtInventory`))
  (bind _currentfisharea (`self.CurrentFishArea`))
  (bind _currentfisharea_2 (`self.CurrentFishArea`))
  (bind _bobberref (`self.BobberRef`))
  (bind _currentfisharea_3 (`self.CurrentFishArea`))
  (bind _hookedhandle (`self.HookedHandle`))
  (bind _bobber (`/Game/Blueprints/FishStuff/FishArea.Bobber` (`self.CurrentFishArea`)))
  (bind _returnvalue (`self.K2_GetActorLocation` (`/Game/Blueprints/FishStuff/FishArea.Bobber` (`self.CurrentFishArea`))))
  (bind _movespeed (`/Game/Blueprints/FishStuff/FishableItems/FishableItemOB.MoveSpeed` (`/Game/Blueprints/FishStuff/FishArea.ItemObj` _currentfisharea)))
  (bind _returnvalue_2 (- (`/Game/Blueprints/FishingPoles/FishingPole.Pullspeed` (`self.CurrentPole`)) _movespeed))
  (bind (_returnvalue_x_2 _returnvalue_y_2) (`KismetMathLibrary.BreakVector` (`KismetMathLibrary.Normal` (- _returnvalue (`self.K2_GetActorLocation`)))))
  (bind (_returnvalue_x_3 _returnvalue_y_3) (`KismetMathLibrary.BreakVector` (`KismetMathLibrary.Normal` (- (`self.K2_GetActorLocation` (`/Game/Blueprints/FishStuff/FishArea.Bobber` (`self.CurrentFishArea`))) (`self.K2_GetActorLocation`)))))
  (bind _returnvalue_3 (`KismetMathLibrary.Vector_Distance` (`KismetMathLibrary.MakeVector` _returnvalue_x _returnvalue_y) (`KismetMathLibrary.MakeVector` (.x _returnvalue) (.y _returnvalue))))
  (bind _returnvalue_4 (`KismetMathLibrary.Dot_VectorVector` (`KismetMathLibrary.Normal` (+ (`self.ReelForward`) (`self.ReelRight`))) (`KismetMathLibrary.MakeVector` _returnvalue_x_2 _returnvalue_y_2)))
  (if (< _returnvalue_3 100.0)
    (`KismetArrayLibrary.Array_Add` _caughtinventory (`/Game/Blueprints/FishStuff/FishArea.ItemObj` _currentfisharea_3))
    (`KismetSystemLibrary.PrintString` (`KismetStringLibrary.Conv_IntToString` (`KismetArrayLibrary.Array_Length` _caughtinventory)))
    (`/Game/Blueprints/FishStuff/FishArea.Clear all timers` _currentfisharea_3)
    (`self.K2_DestroyActor` _currentfisharea_2)
    (`self.K2_DestroyActor` _bobberref)
    (set `self.Hooked` false)
    (set `self.IsFishing` false)
    (set `self.CanMove` true)
    (`KismetSystemLibrary.K2_ClearAndInvalidateTimerHandle` _hookedhandle)
    (elif (> _returnvalue_3 2000.0)
      (`/Game/Blueprints/FishStuff/FishArea.Clear all timers` _currentfisharea_3)
      (if (`/Game/Blueprints/FishStuff/FishArea.fishingSpotDissapear` (`self.CurrentFishArea`))
        (`self.K2_DestroyActor` _currentfisharea_2)
        (`self.K2_DestroyActor` _bobberref)
        (set `self.Hooked` false)
        (set `self.IsFishing` false)
        (set `self.CanMove` true)
        (`KismetSystemLibrary.K2_ClearAndInvalidateTimerHandle` _hookedhandle)
        (else
          (`self.K2_DestroyActor` _bobberref)
          (set `self.Hooked` false)
          (set `self.IsFishing` false)
          (set `self.CanMove` true)
          (`KismetSystemLibrary.K2_ClearAndInvalidateTimerHandle` _hookedhandle)))
      (elif (< _returnvalue_2 0.0)
        (set `/Game/Blueprints/FishStuff/FishArea.CurrentMoveSpeed` (- (`/Game/Blueprints/FishStuff/FishableItems/FishableItemOB.MoveSpeed` (`/Game/Blueprints/FishStuff/FishArea.ItemObj` (`self.CurrentFishArea`))) (`/Game/Blueprints/FishingPoles/FishingPole.Pullspeed` (`self.CurrentPole`))) _currentfisharea)
        (elif (< _returnvalue_4 -0.7)
          (set `/Game/Blueprints/FishStuff/FishArea.CurrentMoveSpeed` 0.0 _currentfisharea)
          (if (< _returnvalue_3 400.0)
            (set `local.ReelDir` (`KismetMathLibrary.Normal` (- (`self.K2_GetActorLocation` (`/Game/Blueprints/FishStuff/FishArea.Bobber` (`self.CurrentFishArea`))) (`self.K2_GetActorLocation`))))
            (else
              (set `local.ReelDir` (`KismetMathLibrary.MakeVector` _returnvalue_x_3 _returnvalue_y_3))))
          (`self.K2_SetActorLocation` _bobber (+ (* (`local.ReelDir`) (* _returnvalue_4 _returnvalue_2)) (`self.K2_GetActorLocation` _bobber)) true false)
          (else
            (set `/Game/Blueprints/FishStuff/FishArea.CurrentMoveSpeed` _movespeed _currentfisharea)))))))

(fn `StartHooked`
  (set `self.Hooked` true)
  (bind _returnvalue (`KismetSystemLibrary.K2_SetTimer` null "Reel Hooked" 0.001 true))
  (set `self.HookedHandle` _returnvalue)
  (`KismetSystemLibrary.K2_ClearAndInvalidateTimerHandle` (`self.ReelHandle`)))

(fn `UserConstructionScript`
  (`SceneComponent.SetAbsolute` (`self.SpringArm`) false true false))
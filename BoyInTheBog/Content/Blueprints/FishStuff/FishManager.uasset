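; FishManager seeds fishing spots around the player's boat when play begins.
; On BeginPlay it finds the BP_Boat, then spawns several FishArea actors at random navigable points within a large radius of it, flattened to zero height.
; Each area is initialized with TestFish and added to FishableAreas; the random pick from SpawnableFishableItems and the stored nav mesh bounds volume are unused.
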(event `self.ReceiveBeginPlay`
  (bind _returnvalue (`GameplayStatics.GetActorOfClass` "/Script/NavigationSystem.NavMeshBoundsVolume"))
  (set `self.NavMesh` _returnvalue)
  (bind _returnvalue_2 (`GameplayStatics.GetActorOfClass` "/Game/Blueprints/BP_Boat.BP_Boat_C"))
  (set `self.Boat` _returnvalue_2)
  (for _ (range 7)
    (`self.Randomly Spawn Fish Group` 10000.0)))

(fn `Randomly Spawn Fish Group`
  (params (SpawnRadius :type "Float (double-precision)"))
  (bind _randomlocation (`NavigationSystemV1.K2_GetRandomLocationInNavigableRadius` (`self.K2_GetActorLocation` (`self.Boat`)) SpawnRadius (`self.NavData`) null))
  (bind _returnvalue (`|SpawnActorFromClass` "/Game/Blueprints/FishStuff/FishArea.FishArea_C" (`KismetMathLibrary.MakeTransform` (`KismetMathLibrary.MakeVector` (.x _randomlocation) (.y _randomlocation))) "Undefined" "OverrideRootScale" null null))
  (`/Game/Blueprints/FishStuff/FishArea.InitializeSpot` _returnvalue "/Game/Blueprints/FishStuff/FishableItems/TestFish.TestFish_C")
  (`KismetArrayLibrary.Array_Add` (`self.FishableAreas`) _returnvalue))

(fn `UserConstructionScript`)
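; FishArea is a fishing spot that holds a constructed item object and drives its direction changes once hooked.
; InitializeSpot creates the item; StartHooked loops HookedBehavior and ChooseNewDirection timers, randomly offsetting the item's switch time by its deviation.
; ChooseNewDirection re-rolls random flat directions until one does not point away from the game mode's Boy, then prints it.
; HookedBehavior, Move and RechargeStamina are empty stubs.
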(event `self.ReceiveBeginPlay`
  (bind _asbp_bbgame_mode (cast `/Game/Blueprints/BP_BBGameMode` (`GameplayStatics.GetGameMode`)))
  (set `self.As BP BBGame Mode` _asbp_bbgame_mode))

(fn `ChooseNewDirection`
  (set `self.Direction` (`KismetMathLibrary.Normal` (`KismetMathLibrary.MakeVector` (`KismetMathLibrary.RandomFloatInRange` -1.0 1.0) (`KismetMathLibrary.RandomFloatInRange` -1.0 1.0))))
  (while (< (`KismetMathLibrary.Dot_VectorVector` (`KismetMathLibrary.Normal` (- (`self.K2_GetActorLocation` (`/Game/Blueprints/BP_BBGameMode.Boy` (`self.As BP BBGame Mode`))) (`self.K2_GetActorLocation`))) (`self.Direction`)) 0.0)
    (set `self.Direction` (`KismetMathLibrary.Normal` (`KismetMathLibrary.MakeVector` (`KismetMathLibrary.RandomFloatInRange` -1.0 1.0) (`KismetMathLibrary.RandomFloatInRange` -1.0 1.0)))))
  (`KismetSystemLibrary.PrintString` (`KismetStringLibrary.Conv_VectorToString` (`self.Direction`))))

(fn `HookedBehavior`)

(fn `InitializeSpot`
  (params (ItemToMake :type "/Game/Blueprints/FishStuff/FishableItems/FishableItemOB Class Reference"))
  (bind _returnvalue (`|GenericCreateObject` ItemToMake self))
  (set `self.ItemObj` _returnvalue))

(fn `Move`)

(fn `RechargeStamina`)

(fn `StartHooked`
  (bind _itemobj (`self.ItemObj`))
  (bind _itemobj_2 (`self.ItemObj`))
  (bind _returnvalue (`KismetSystemLibrary.K2_SetTimer` null "HookedBehavior" 0.001 true))
  (set `self.Hooked Handle` _returnvalue)
  (switch `int` (`KismetMathLibrary.RandomInteger` 2)
    (:`0`
      (set `self.NewDirectionTime` (`KismetMathLibrary.FClamp` (+ (`/Game/Blueprints/FishStuff/FishableItems/FishableItemOB.SwitchTime` _itemobj_2) (`/Game/Blueprints/FishStuff/FishableItems/FishableItemOB.SwitchTimeDerrivation` _itemobj_2)) 0.0 10.0)))
    (:`1`
      (set `self.NewDirectionTime` (`KismetMathLibrary.FClamp` (- (`/Game/Blueprints/FishStuff/FishableItems/FishableItemOB.SwitchTime` _itemobj) (`/Game/Blueprints/FishStuff/FishableItems/FishableItemOB.SwitchTimeDerrivation` _itemobj)) 0.0 10.0))))
  (bind _returnvalue_2 (`KismetSystemLibrary.K2_SetTimer` null "ChooseNewDirection" (`self.NewDirectionTime`) true))
  (set `self.NewDirectionHandle` _returnvalue_2))

(fn `UserConstructionScript`)
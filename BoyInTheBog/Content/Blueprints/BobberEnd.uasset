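; BobberEnd is the end of a fishing bobber, using its Box overlap to start a hooked sequence and detect a catch.
; When not fishing, overlapping a FishArea registers the bobber with it, sets it as the Boy's current area through BP_BBGameMode, and calls StartHooked on both.
; It then flags itself as Fishing, so any later overlap, whatever the actor, marks it Caught.
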(event `self.ReceiveBeginPlay`
  (bind _asbp_bbgame_mode (cast `/Game/Blueprints/BP_BBGameMode` (`GameplayStatics.GetGameMode`)))
  (set `self.GamemodeRef` _asbp_bbgame_mode))

(event `self.Box.OnComponentBeginOverlap`
  (params (OverlappedComponent :type "PrimitiveComponent Object Reference") (OtherActor :type "Actor Object Reference") (OtherComp :type "PrimitiveComponent Object Reference") (OtherBodyIndex :type Integer) (bFromSweep :type Boolean) (SweepResult :type "HitResult Structure (by ref)"))
  (bind _boy (`/Game/Blueprints/BP_BBGameMode.Boy` (`self.GamemodeRef`)))
  (if (`self.fishing`)
    (set `self.Caught` true)
    (else
      (bind _asfish_area (cast `/Game/Blueprints/FishStuff/FishArea` OtherActor))
      (set `/Game/Blueprints/FishStuff/FishArea.Bobber` self _asfish_area)
      (set `/Game/Blueprints/BP_Boy.CurrentFishArea` _asfish_area _boy)
      (`/Game/Blueprints/FishStuff/FishArea.StartHooked` _asfish_area)
      (`/Game/Blueprints/BP_Boy.StartHooked` _boy)
      (set `self.fishing` true))))

(fn `UserConstructionScript`)